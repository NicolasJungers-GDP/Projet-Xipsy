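; BP_cristaux is a puzzle Blueprint that swaps visibility between two crystal components, Cristal and Cristal1.
; On BeginPlay it hides Cristal and sets a boolean that is not read in these graphs.
; Overlapping Box shows Cristal and hides Cristal1, while overlapping Box1 does the reverse.
; The overlap events apply no actor filter, and the visibility changes do not propagate to child components.
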(event OnComponentBeginOverlap(Box)
  (params (OverlappedComponent :type Primitive%20Component%20Object%20Reference) (OtherActor :type Actor%20Object%20Reference) (OtherComp :type Primitive%20Component%20Object%20Reference) (OtherBodyIndex :type Integer) (bFromSweep :type Boolean) (SweepResult :type Hit%20Result%20Structure%20%28by%20ref%29))
  (Rendering|SetVisibility (Variables|Default|Getcristal1) false false)
  (Rendering|SetVisibility (Variables|Default|Getcristal) true false))

(event OnComponentBeginOverlap(Box1)
  (params (OverlappedComponent :type Primitive%20Component%20Object%20Reference) (OtherActor :type Actor%20Object%20Reference) (OtherComp :type Primitive%20Component%20Object%20Reference) (OtherBodyIndex :type Integer) (bFromSweep :type Boolean) (SweepResult :type Hit%20Result%20Structure%20%28by%20ref%29))
  (Rendering|SetVisibility (Variables|Default|Getcristal) false false)
  (Rendering|SetVisibility (Variables|Default|Getcristal1) true false))

(event EventBeginPlay
  (Variables|Default|SetNewVar_0 true)
  (Rendering|SetVisibility (Variables|Default|Getcristal) false false))

(fn ConstructionScript)