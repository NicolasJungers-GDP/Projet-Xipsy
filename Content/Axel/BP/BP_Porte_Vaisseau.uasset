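; Spaceship door actor that slides its door mesh slightly down in relative space, then back up to close automatically.
; BeginPlay caches both door transforms, and third-person character overlaps with the Box open or close a Gate node.
; The Gate's exit plays a sound and an opening timeline that lerps the transform.
; When it finishes, a second timeline immediately plays in reverse to return the door.
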(event OnComponentBeginOverlap(Box)
  (params (OverlappedComponent :type Primitive%20Component%20Object%20Reference) (OtherActor :type Actor%20Object%20Reference) (OtherComp :type Primitive%20Component%20Object%20Reference) (OtherBodyIndex :type Integer) (bFromSweep :type Boolean) (SweepResult :type Hit%20Result%20Structure%20%28by%20ref%29))
  (Utilities|Casting|CastToBP_ThirdPersonCharacter OtherActor)
  (Utilities|FlowControl|Gate true ; enters at Open
    (:Exit
      (Audio|PlaySoundatLocation 0 (Transformation|GetActorLocation) "0, 0, 0" 1.0 1.0 0.0 0 0 0 0)
      (bind _open_door (Timeline|Open%20Door Play)
        (:Update
          (Transformation|SetRelativeTransform (Variables|Default|GetVaisseau_3_Vaisseau_Porte_D_Porte) (Math|Transform|Lerp(Transform) (Variables|Default|GetOut%20Position) (Variables|Default|GetIn%20Position) _open_door) false false))
        (:Finished
          (bind _open_door_2 (Timeline|Timeline_0 ReverseFromEnd)
            (:Update
              (Transformation|SetRelativeTransform (Variables|Default|GetVaisseau_3_Vaisseau_Porte_D_Porte) (Math|Transform|Lerp(Transform) (Variables|Default|GetOut%20Position) (Variables|Default|GetIn%20Position) _open_door_2) false false))))))))

(event OnComponentEndOverlap(Box)
  (params (OverlappedComponent :type Primitive%20Component%20Object%20Reference) (OtherActor :type Actor%20Object%20Reference) (OtherComp :type Primitive%20Component%20Object%20Reference) (OtherBodyIndex :type Integer))
  (Utilities|Casting|CastToBP_ThirdPersonCharacter OtherActor)
  (Utilities|FlowControl|Gate true ; enters at Close
    (:Exit
      (Audio|PlaySoundatLocation 0 (Transformation|GetActorLocation) "0, 0, 0" 1.0 1.0 0.0 0 0 0 0)
      (bind _open_door (Timeline|Open%20Door Play)
        (:Update
          (Transformation|SetRelativeTransform (Variables|Default|GetVaisseau_3_Vaisseau_Porte_D_Porte) (Math|Transform|Lerp(Transform) (Variables|Default|GetOut%20Position) (Variables|Default|GetIn%20Position) _open_door) false false))
        (:Finished
          (bind _open_door_2 (Timeline|Timeline_0 ReverseFromEnd)
            (:Update
              (Transformation|SetRelativeTransform (Variables|Default|GetVaisseau_3_Vaisseau_Porte_D_Porte) (Math|Transform|Lerp(Transform) (Variables|Default|GetOut%20Position) (Variables|Default|GetIn%20Position) _open_door_2) false false))))))))

(event EventBeginPlay
  (bind _vaisseau_3_vaisseau_porte_d_porte (Variables|Default|GetVaisseau_3_Vaisseau_Porte_D_Porte))
  (bind _returnvalue (Transformation|GetRelativeTransform _vaisseau_3_vaisseau_porte_d_porte))
  (Variables|Default|SetOut%20Position (Math|Transform|MakeTransform (.location _returnvalue) (.rotation _returnvalue) (.scale _returnvalue)))
  (Variables|Default|SetIn%20Position (Math|Transform|MakeTransform (- (.location _returnvalue) "0,0.000000,10.000000") (.rotation _returnvalue) (.scale _returnvalue)))
  (Input|EnableInput (Game|GetPlayerController 0)))

(fn ConstructionScript)