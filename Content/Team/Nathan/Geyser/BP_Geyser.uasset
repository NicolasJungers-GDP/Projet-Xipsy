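; BP_Geyser is a geyser that launches the third-person player character while it stands inside the Box trigger.
; Overlap events set an in-box flag, and Tick launches along the Arrow's forward vector, scaled by separate horizontal and vertical forces, overriding velocity.
; Delays on Tick toggle the launch flag between active and cooldown periods.
; The construction script pitches the Arrow to a configurable angle using the actor's yaw.
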(event OnComponentBeginOverlap(Box)
  (params (OverlappedComponent :type Primitive%20Component%20Object%20Reference) (OtherActor :type Actor%20Object%20Reference) (OtherComp :type Primitive%20Component%20Object%20Reference) (OtherBodyIndex :type Integer) (bFromSweep :type Boolean) (SweepResult :type Hit%20Result%20Structure%20%28by%20ref%29))
  (Utilities|Casting|CastToBP_ThirdPersonCharacter OtherActor)
  (Variables|Launch|SetIsInBox true))

(event OnComponentEndOverlap(Box)
  (params (OverlappedComponent :type Primitive%20Component%20Object%20Reference) (OtherActor :type Actor%20Object%20Reference) (OtherComp :type Primitive%20Component%20Object%20Reference) (OtherBodyIndex :type Integer))
  (Utilities|Casting|CastToBP_ThirdPersonCharacter OtherActor)
  (Variables|Launch|SetIsInBox false))

(event EventTick
  (params (DeltaSeconds :type Float%20%28single-precision%29))
  (bind _hforce (Variables|Launch|GetHForce))
  (if (Variables|Launch|GetIsInBox)
    (bind _asbp_third_person_character (Utilities|Casting|CastToBP_ThirdPersonCharacter (Game|GetPlayerCharacter 0)))
    (if (Variables|Launch|GetLaunchActif)
      (Character|LaunchCharacter _asbp_third_person_character (* (Math|Vector|GetForwardVector (Variables|Default|GetArrow)) (Math|Vector|MakeVector _hforce _hforce (Variables|Launch|GetVForce))) true true)
      (Variables|Launch|SetLaunchActif true)
      (Utilities|FlowControl|Delay (Variables|Launch|GetTimeActif))
      (Variables|Launch|SetLaunchActif false)
      (Utilities|FlowControl|Delay (Variables|Launch|GetTimeCoolDown))
      (Variables|Launch|SetLaunchActif true))))

(fn ConstructionScript
  (Transformation|SetWorldRotation (Variables|Default|GetArrow) (Math|Rotator|MakeRotator 0.0 (Variables|Launch|GetAngle) (.yaw (Transformation|GetActorRotation))) false false))