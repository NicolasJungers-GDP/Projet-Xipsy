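; BP_Xipsy is a quest-giver NPC that offers dialogue and shows quest state through exclamation and question marks.
; An overlap box shows the chat prompt; ActivateDialogue removes a completed quest from the player, then opens an NPC_Dialogue widget.
; A brief black screen masks the switch to the NPC camera and player teleport to the Cone, both placed by the construction script.
; EndChat blends back to the player camera and restores control.
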(event OnComponentBeginOverlap(Box)
  (params (OverlappedComponent :type Primitive%20Component%20Object%20Reference) (OtherActor :type Actor%20Object%20Reference) (OtherComp :type Primitive%20Component%20Object%20Reference) (OtherBodyIndex :type Integer) (bFromSweep :type Boolean) (SweepResult :type Hit%20Result%20Structure%20%28by%20ref%29))
  ;[1 1 1] Voir "Press "E" to chat"
  (Utilities|Casting|CastToBP_ThirdPersonCharacter OtherActor)
  (Development|SetHiddeninGame (Variables|Default|GetTextRender) false false))

(event OnComponentEndOverlap(Box)
  (params (OverlappedComponent :type Primitive%20Component%20Object%20Reference) (OtherActor :type Actor%20Object%20Reference) (OtherComp :type Primitive%20Component%20Object%20Reference) (OtherBodyIndex :type Integer))
  ;[1 1 1] Voir "Press "E" to chat"
  (Utilities|Casting|CastToBP_ThirdPersonCharacter OtherActor)
  (Development|SetHiddeninGame (Variables|Default|GetTextRender) true false))

(event Custom|BeginChat
  (bind _npcchat (Variables|Default|GetNPCChat))
  ;[1 1 1] Commencer à parler
  (Default|Begin _npcchat (Variables|Default|GetConversationInfo))
  (UserInterface|Viewport|AddtoViewport _npcchat 0))

(event Custom|PlayerAdjustments
  (bind _returnvalue (Game|GetPlayerCharacter 0))
  (bind _cone (Variables|Default|GetCone))
  (bind _returnvalue_2 (Transformation|GetWorldLocation _cone))
  (bind _rootcomponent (Variables|/Script/Engine.Actor|GetRootComponent _returnvalue))
  (bind _returnvalue_3 (Transformation|GetWorldRotation _rootcomponent))
  ;[1 1 1] Mouvement de caméra + fade en noir
  (Variables|/Script/Engine.PlayerController|SetbShowMouseCursor (Game|GetPlayerController 0) true)
  (Pawn|Components|CharacterMovement|DisableMovement (Variables|/Script/Engine.Character|GetCharacterMovement (Game|GetPlayerCharacter 0)))
  (Input|SetInputModeUIOnly (Game|GetPlayerController 0) 0 "DoNotLock")
  (bind _returnvalue_4 (UserInterface|CreateWidget "/Game/Nathan/Dialogue_Quests/BlackScreenPop.BlackScreenPop_C"))
  (UserInterface|Viewport|AddtoViewport _returnvalue_4 0)
  (Utilities|FlowControl|Delay 0.2)
  (Game|Player|SetViewTargetwithBlend (Game|GetPlayerController 0) (Components|GetOwner (Variables|Default|GetCamera)) 0.0 "VTBlend_Linear" 0.0 false)
  (Transformation|SetWorldTransform (Variables|/Script/Engine.Actor|GetRootComponent (Game|GetPlayerCharacter 0)) (Math|Transform|MakeTransform (Math|Vector|MakeVector (.x _returnvalue_2) (.y _returnvalue_2) (.z (Transformation|GetWorldLocation (Variables|/Script/Engine.Actor|GetRootComponent (Game|GetPlayerCharacter 0))))) (Math|Rotator|MakeRotator (.roll _returnvalue_3) (.pitch _returnvalue_3) (+ (.yaw (Transformation|GetWorldRotation (Variables|Character|GetMesh))) -9e+01)) "1.000000,1.000000,1.000000") false false)
  (Utilities|FlowControl|Delay 0.2)
  (Widget|RemovefromParent _returnvalue_4))

(event Custom|EventQuestComplete
  ;[1 1 1] Quête Finie
  (Variables|/Game/Nathan/Dialogue_Quests/NPC_Dialogue.NPC_Dialogue_C|SetQuestFinished (Variables|Default|GetNPCChat) true)
  (Rendering|Material|SetMaterial (Variables|Default|GetQuestionMark) 0 "/Game/Nathan/Dialogue_Quests/QuestComplete_Mat.QuestComplete_Mat")
  (Variables|Default|SetQuestComplete true))

(event Custom|EndChat
  (bind _returnvalue (Game|GetPlayerController 0))
  ;[1 1 1] Finir de parler
  (Widget|RemovefromParent (Variables|Default|GetNPCChat))
  (Game|Player|SetViewTargetwithBlend (Game|GetPlayerController 0) (Components|GetOwner (Variables|/Game/ThirdPerson/Blueprints/BP_ThirdPersonCharacter.BP_ThirdPersonCharacter_C|GetFollowCamera (.AsBP%20Third%20Person%20Character (Utilities|Casting|CastToBP_ThirdPersonCharacter (Game|GetPlayerCharacter 0))))) 1.3 "VTBlend_Linear" 0.0 false)
  (Utilities|FlowControl|Delay 1.3)
  (Input|SetInputModeGameOnly _returnvalue)
  (Variables|/Script/Engine.PlayerController|SetbShowMouseCursor _returnvalue false)
  (Pawn|Components|CharacterMovement|SetMovementMode (Variables|/Script/Engine.Character|GetCharacterMovement (Game|GetPlayerCharacter 0)) "MOVE_Walking" 0))

(event Custom|AcceptQuest
  ;[1 1 1] Quête accepté
  (Development|SetHiddeninGame (Variables|Default|GetQuestionMark) false false)
  (Development|SetHiddeninGame (Variables|Default|GetExclamationMark) true false)
  (bind _asbp_third_person_character (Utilities|Casting|CastToBP_ThirdPersonCharacter (Game|GetPlayerCharacter 0)))
  (Default|AcceptQuest _asbp_third_person_character (Variables|Default|GetQuestRef))
  (Variables|Default|SetQuestActive? true))

(event EventBeginPlay
  ;[1 1 1] Créer le widget pour le chat
  (bind _returnvalue (UserInterface|CreateWidget "/Game/Nathan/Dialogue_Quests/NPC_Dialogue.NPC_Dialogue_C"))
  (bind _output_get (Variables|Default|SetNPCChat _returnvalue))
  (Variables|/Game/Nathan/Dialogue_Quests/NPC_Dialogue.NPC_Dialogue_C|SetNPC_Ref _output_get self)
  (Utilities|IsValid (.actorreference (Variables|Default|GetQuestRef))
    (:Is%20Valid
      (Development|SetHiddeninGame (Variables|Default|GetExclamationMark) false false))))

(event EventActivateDialogue
  (params (QuestLogInfo :type Array%20of%20BP%20Quest%20Object%20References))
  ;[1 1 1] Interagir
  (CallFunction|PlayerAdjustments)
  (Development|SetHiddeninGame (Variables|Default|GetTextRender) true false)
  (if (Variables|Default|GetQuestActive?)
    (for _array_element QuestLogInfo
      (if (Utilities|Enum|Equal(Enum) (.questname (Variables|/Game/Nathan/Dialogue_Quests/BP_Quest.BP_Quest_C|GetQuestInfo _array_element)) (.QuestName (Utilities|Struct|BreakQuestInfo (Variables|Default|GetQuestRef))))
        (if (Variables|Default|GetQuestComplete)
          (bind _asbp_third_person_character (Utilities|Casting|CastToBP_ThirdPersonCharacter (Game|GetPlayerCharacter 0)))
          (Default|RemoveQuest _asbp_third_person_character _array_element)
          (Development|SetHiddeninGame (Variables|Default|GetQuestionMark) true false)))))
  (Utilities|FlowControl|Delay 0.2)
  (CallFunction|BeginChat))

(fn ConstructionScript
  (Transformation|SetRelativeTransform (Variables|Default|GetCamera) (Variables|Default|GetCameraTransform) false false)
  (Transformation|SetRelativeLocation (Variables|Default|GetCone) (Variables|Default|GetPlayerLocation) false false))

(fn ReturnCameraPlayer
  (Game|Player|SetViewTargetwithBlend (Game|GetPlayerController 0) self 1.0 "VTBlend_Linear" 0.0 false)
  (Pawn|Components|CharacterMovement|SetMovementMode (Variables|Character|GetCharacterMovement) "MOVE_Walking" 0))