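; SparkBP is an interactable actor that shows a spark and sends it along a spline path.
; A box overlap with the third-person character enables input and opens a gate for the Interact press.
; Interact reveals the spark, grabs a SplinePathBP via GetActorOfClass, and runs a timeline scaled by TimeToComplete.
; The timeline moves the whole actor along the spline (world location, local rotation), then hides the spark.
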(event OnComponentBeginOverlap(Box)
  (params (OverlappedComponent :type Primitive%20Component%20Object%20Reference) (OtherActor :type Actor%20Object%20Reference) (OtherComp :type Primitive%20Component%20Object%20Reference) (OtherBodyIndex :type Integer) (bFromSweep :type Boolean) (SweepResult :type Hit%20Result%20Structure%20%28by%20ref%29))
  (Utilities|Casting|CastToBP_ThirdPersonCharacter OtherActor)
  (Input|EnableInput (Game|GetPlayerController 0))
  (Utilities|FlowControl|Gate true) ; enters at Open
)

(event OnComponentEndOverlap(Box)
  (params (OverlappedComponent :type Primitive%20Component%20Object%20Reference) (OtherActor :type Actor%20Object%20Reference) (OtherComp :type Primitive%20Component%20Object%20Reference) (OtherBodyIndex :type Integer))
  (Utilities|Casting|CastToBP_ThirdPersonCharacter OtherActor)
  (Input|DisableInput (Game|GetPlayerController 0))
  (Utilities|FlowControl|Gate true) ; enters at Close
)

(event Custom|MoveObject
  (bind _splineref (Variables|Default|GetSplineRef))
  (bind _spline (Variables|/Game/Nathan/SplinePathBP.SplinePathBP_C|GetSpline _splineref))
  (Components|Timeline|SetPlayRate (Variables|Default|GetMoveObjectT) (/ 1.0 (Variables|Default|GetTimeToComplete)))
  (bind _movetrack (Timeline|MoveObjectT Play)
    (:Update
      (Transformation|SetActorTransform (Math|Transform|MakeTransform (Spline|GetLocationatDistanceAlongSpline _spline (Math|Float|Lerp 0.0 (Spline|GetSplineLength (Variables|/Game/Nathan/SplinePathBP.SplinePathBP_C|GetSpline (Variables|Default|GetSplineRef))) _movetrack) "World") (Spline|GetRotationatDistanceAlongSpline _spline (Math|Float|Lerp 0.0 (Spline|GetSplineLength (Variables|/Game/Nathan/SplinePathBP.SplinePathBP_C|GetSpline (Variables|Default|GetSplineRef))) _movetrack) "Local") "1.000000,1.000000,1.000000")))
    (:Finished
      (Development|SetHiddeninGame (Variables|Default|GetP_Spark) true false))))

(event EventBeginPlay
  (Development|SetHiddeninGame (Variables|Default|GetP_Spark) true false))

(event Input|ActionEvents|InputActionInteract
  (params (Key :type Key%20Structure :default "None"))
  (:Pressed
    (Utilities|FlowControl|Gate true
      (:Exit
        (Development|SetHiddeninGame (Variables|Default|GetP_Spark) false false)
        (bind _returnvalue (Actor|GetActorOfClass "/Game/Nathan/SplinePathBP.SplinePathBP_C"))
        (Variables|Default|SetSplineRef _returnvalue)
        (CallFunction|MoveObject)))))

(fn ConstructionScript)