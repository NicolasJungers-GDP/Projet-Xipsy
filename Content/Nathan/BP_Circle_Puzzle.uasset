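; Interactive puzzle actor where the player rotates three concentric-style circle meshes from a dedicated camera.
; A trigger box enables input and gates Interact, which toggles the blended puzzle camera and character movement.
; Up/Down select and highlight a circle, while Left/Right turn it 90 degrees via timelines, locking input until finished.
; Tick copies the follow camera's yaw and roll onto the puzzle camera; PuzzleSolved blocks entry but is never set here.
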(event OnComponentBeginOverlap(Box)
  (params (OverlappedComponent :type Primitive%20Component%20Object%20Reference) (OtherActor :type Actor%20Object%20Reference) (OtherComp :type Primitive%20Component%20Object%20Reference) (OtherBodyIndex :type Integer) (bFromSweep :type Boolean) (SweepResult :type Hit%20Result%20Structure%20%28by%20ref%29))
  ;[1 1 1] Transition de caméra
  (Utilities|Casting|CastToBP_ThirdPersonCharacter OtherActor)
  (Input|EnableInput (Game|GetPlayerController 0))
  (Utilities|FlowControl|Gate true) ; enters at Open
)

(event OnComponentEndOverlap(Box)
  (params (OverlappedComponent :type Primitive%20Component%20Object%20Reference) (OtherActor :type Actor%20Object%20Reference) (OtherComp :type Primitive%20Component%20Object%20Reference) (OtherBodyIndex :type Integer))
  ;[1 1 1] Transition de caméra
  (Utilities|Casting|CastToBP_ThirdPersonCharacter OtherActor)
  (Input|DisableInput (Game|GetPlayerController 0))
  (Utilities|FlowControl|Gate true) ; enters at Close
)

(event Custom|TurnCircleLeft
  (params (Circle :type Scene%20Component%20Object%20Reference) (Circle2 :type Scene%20Component%20Object%20Reference) (Circle3 :type Scene%20Component%20Object%20Reference))
  (bind _returnvalue (Transformation|GetWorldRotation Circle3))
  (bind _returnvalue_2 (Transformation|GetWorldRotation Circle))
  (bind _returnvalue_3 (Transformation|GetWorldRotation Circle2))
  (Utilities|FlowControl|Sequence
    (:then_0
      (Utilities|IsValid Circle
        (:Is%20Valid
          (Variables|Default|SetMechanismZ_1 (.yaw _returnvalue_2))
          (bind _alpha (Timeline|Timeline_0 PlayFromStart)
            (:Update
              (Transformation|SetRelativeRotation Circle (Math|Rotator|Lerp(Rotator) (Math|Rotator|MakeRotator (.roll _returnvalue_2) (.pitch _returnvalue_2) (Variables|Default|GetMechanismZ_1)) (Math|Rotator|MakeRotator (.roll _returnvalue_2) (.pitch _returnvalue_2) (- (Variables|Default|GetMechanismZ_1) 9e+01)) _alpha) false false))
            (:Finished
              (Variables|Default|SetRotating false))))))
    (:then_1
      (Utilities|IsValid Circle2
        (:Is%20Valid
          (Variables|Default|SetMechanismZ_2 (.yaw _returnvalue_3))
          (bind _alpha_2 (Timeline|Timeline_1 PlayFromStart)
            (:Update
              (Transformation|SetRelativeRotation Circle2 (Math|Rotator|Lerp(Rotator) (Math|Rotator|MakeRotator (.roll _returnvalue_3) (.pitch _returnvalue_3) (Variables|Default|GetMechanismZ_2)) (Math|Rotator|MakeRotator (.roll _returnvalue_3) (.pitch _returnvalue_3) (- (Variables|Default|GetMechanismZ_2) 9e+01)) _alpha_2) false false))
            (:Finished
              (Variables|Default|SetRotating false))))))
    (:then_2
      (Utilities|IsValid Circle3
        (:Is%20Valid
          (Variables|Default|SetMechanismZ_3 (.yaw _returnvalue))
          (bind _alpha_3 (Timeline|Timeline_2 PlayFromStart)
            (:Update
              (Transformation|SetRelativeRotation Circle3 (Math|Rotator|Lerp(Rotator) (Math|Rotator|MakeRotator (.roll _returnvalue) (.pitch _returnvalue) (Variables|Default|GetMechanismZ_3)) (Math|Rotator|MakeRotator (.roll _returnvalue) (.pitch _returnvalue) (- (Variables|Default|GetMechanismZ_3) 9e+01)) _alpha_3) false false))
            (:Finished
              (Variables|Default|SetRotating false))))))))

(event Custom|TurnCircleRight
  (params (Circle :type Scene%20Component%20Object%20Reference) (Circle2 :type Scene%20Component%20Object%20Reference) (Circle3 :type Scene%20Component%20Object%20Reference))
  (bind _returnvalue (Transformation|GetWorldRotation Circle))
  (bind _returnvalue_2 (Transformation|GetWorldRotation Circle2))
  (bind _returnvalue_3 (Transformation|GetWorldRotation Circle3))
  (Utilities|FlowControl|Sequence
    (:then_0
      (Utilities|IsValid Circle
        (:Is%20Valid
          (Variables|Default|SetMechanismZ_1 (.yaw _returnvalue))
          (bind _alpha (Timeline|Circle1Right PlayFromStart)
            (:Update
              (Transformation|SetRelativeRotation Circle (Math|Rotator|Lerp(Rotator) (Math|Rotator|MakeRotator (.roll _returnvalue) (.pitch _returnvalue) (Variables|Default|GetMechanismZ_1)) (Math|Rotator|MakeRotator (.roll _returnvalue) (.pitch _returnvalue) (+ (Variables|Default|GetMechanismZ_1) 9e+01)) _alpha) false false))
            (:Finished
              (Variables|Default|SetRotating false))))))
    (:then_1
      (Utilities|IsValid Circle2
        (:Is%20Valid
          (Variables|Default|SetMechanismZ_2 (.yaw _returnvalue_2))
          (bind _alpha_2 (Timeline|Circle2Right PlayFromStart)
            (:Update
              (Transformation|SetRelativeRotation Circle2 (Math|Rotator|Lerp(Rotator) (Math|Rotator|MakeRotator (.roll _returnvalue_2) (.pitch _returnvalue_2) (Variables|Default|GetMechanismZ_2)) (Math|Rotator|MakeRotator (.roll _returnvalue_2) (.pitch _returnvalue_2) (+ (Variables|Default|GetMechanismZ_2) 9e+01)) _alpha_2) false false))
            (:Finished
              (Variables|Default|SetRotating false))))))
    (:then_2
      (Utilities|IsValid Circle3
        (:Is%20Valid
          (Variables|Default|SetMechanismZ_3 (.yaw _returnvalue_3))
          (bind _alpha_3 (Timeline|Circle3Right PlayFromStart)
            (:Update
              (Transformation|SetRelativeRotation Circle3 (Math|Rotator|Lerp(Rotator) (Math|Rotator|MakeRotator (.roll _returnvalue_3) (.pitch _returnvalue_3) (Variables|Default|GetMechanismZ_3)) (Math|Rotator|MakeRotator (.roll _returnvalue_3) (.pitch _returnvalue_3) (+ (Variables|Default|GetMechanismZ_3) 9e+01)) _alpha_3) false false))
            (:Finished
              (Variables|Default|SetRotating false))))))))

(event EventTick
  (params (DeltaSeconds :type Float%20%28single-precision%29))
  (bind _camera (Variables|Default|GetCamera))
  (Utilities|FlowControl|Sequence
    (:then_0
      ;[1 1 1] Récupère la rotation de la caméra du joueur
      (bind _asbp_third_person_character (Utilities|Casting|CastToBP_ThirdPersonCharacter (Game|GetPlayerCharacter 0)))
      (Variables|Default|SetRoationCamera (Transformation|GetWorldRotation (Variables|/Game/ThirdPerson/Blueprints/BP_ThirdPersonCharacter.BP_ThirdPersonCharacter_C|GetFollowCamera _asbp_third_person_character))))
    (:then_1
      (Transformation|SetWorldRotation _camera (Math|Rotator|MakeRotator (.roll (Variables|Default|GetRoationCamera)) (.pitch (Transformation|GetWorldRotation _camera)) (.yaw (Variables|Default|GetRoationCamera))) false false))))

(event Input|ActionEvents|InputActionInteract
  (params (Key :type Key%20Structure :default "None"))
  ;[1 1 1] Transition de caméra
  (:Pressed
    (Utilities|FlowControl|Gate true
      (:Exit
        (Utilities|FlowControl|FlipFlop
          (:A
            (if (not (Variables|Default|GetPuzzleSolved))
              (CallFunction|ProssecPuzzleCamera true)
              (Rendering|Material|SetMaterial (Variables|Default|GetCylinder2) 0 "/Game/Gauthier/Materials/Yellow.Yellow")))
          (:B
            (CallFunction|ProssecPuzzleCamera false)
            (Rendering|Material|SetMaterial (Variables|Default|GetCylinder2) 0 "/Game/Gauthier/Materials/Grey.Grey")
            (Variables|Default|SetSelectCircle 0)))))))

(event Input|KeyboardEvents|Up
  (params (Key :type Key%20Structure :default "None"))
  ;[1 1 1] Selectionner le cercle à bouger
  (:Pressed
    (if (and (not (Variables|Default|GetRotating)) (Variables|Default|GetPuzzleActive?))
      (bind _result (Math|Integer|DecrementInt (Variables|Default|GetSelectCircle))
        (:%20%20
          (Variables|Default|SetSelectCircle (Math|Integer|Clamp(Integer) _result 0 2))
          ;[1 1 1] Séléction du material
          (Rendering|Material|SetMaterial (Variables|Default|GetCylinder2) 0 "/Game/Gauthier/Materials/Grey.Grey")
          (Rendering|Material|SetMaterial (Utilities|Array|Get(acopy) (Utilities|Array|MakeArray (Variables|Default|GetCylinder2) (Variables|Default|GetCylinder1) (Variables|Default|GetCylinder)) (Variables|Default|GetSelectCircle)) 0 "/Game/Gauthier/Materials/Yellow.Yellow"))))))

(event Input|KeyboardEvents|Down
  (params (Key :type Key%20Structure :default "None"))
  ;[1 1 1] Selectionner le cercle à bouger
  (:Pressed
    (if (and (not (Variables|Default|GetRotating)) (Variables|Default|GetPuzzleActive?))
      (bind _result (Math|Integer|IncrementInt (Variables|Default|GetSelectCircle))
        (:%20%20
          (Variables|Default|SetSelectCircle (Math|Integer|Clamp(Integer) _result 0 2))
          ;[1 1 1] Séléction du material
          (Rendering|Material|SetMaterial (Variables|Default|GetCylinder2) 0 "/Game/Gauthier/Materials/Grey.Grey")
          (Rendering|Material|SetMaterial (Utilities|Array|Get(acopy) (Utilities|Array|MakeArray (Variables|Default|GetCylinder2) (Variables|Default|GetCylinder1) (Variables|Default|GetCylinder)) (Variables|Default|GetSelectCircle)) 0 "/Game/Gauthier/Materials/Yellow.Yellow"))))))

(event Input|KeyboardEvents|Left
  (params (Key :type Key%20Structure :default "None"))
  (:Pressed
    (if (and (not (Variables|Default|GetRotating)) (Variables|Default|GetPuzzleActive?))
      (Variables|Default|SetRotating true)
      (switch int (Variables|Default|GetSelectCircle)
        (:0
          (CallFunction|TurnCircleLeft (Variables|Default|GetCylinder2)))
        (:1
          (CallFunction|TurnCircleLeft 0 (Variables|Default|GetCylinder1)))
        (:2
          (CallFunction|TurnCircleLeft 0 0 (Variables|Default|GetCylinder)))))))

(event Input|KeyboardEvents|Right
  (params (Key :type Key%20Structure :default "None"))
  (:Pressed
    (if (and (not (Variables|Default|GetRotating)) (Variables|Default|GetPuzzleActive?))
      (Variables|Default|SetRotating true)
      (switch int (Variables|Default|GetSelectCircle)
        (:0
          (CallFunction|TurnCircleRight (Variables|Default|GetCylinder2)))
        (:1
          (CallFunction|TurnCircleRight 0 (Variables|Default|GetCylinder1)))
        (:2
          (CallFunction|TurnCircleRight 0 0 (Variables|Default|GetCylinder)))))))

(fn ConstructionScript)

(fn ProssecPuzzleCamera
  (params (NewCamera? :type Boolean))
  (bind _output_get (Variables|Default|SetPuzzleActive? NewCamera?))
  (if _output_get
    (Game|Player|SetViewTargetwithBlend (Game|GetPlayerController 0) (Components|GetOwner (Variables|Default|GetCamera)) 1.0 "VTBlend_Linear" 0.0 false)
    (Pawn|Components|CharacterMovement|SetMovementMode (Variables|/Script/Engine.Character|GetCharacterMovement (Game|GetPlayerCharacter 0)) "MOVE_None" 0)
    (Input|SetInputModeGameandUI (Game|GetPlayerController 0) 0 "DoNotLock" true)
    (else
      (Game|Player|SetViewTargetwithBlend (Game|GetPlayerController 0) (Game|GetPlayerCharacter 0) 1.0 "VTBlend_Linear" 0.0 false)
      (Pawn|Components|CharacterMovement|SetMovementMode (Variables|/Script/Engine.Character|GetCharacterMovement (Game|GetPlayerCharacter 0)) "MOVE_Walking" 0)
      (Input|SetInputModeGameOnly (Game|GetPlayerController 0)))))