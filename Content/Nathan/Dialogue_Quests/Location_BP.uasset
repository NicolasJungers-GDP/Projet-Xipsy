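; Location trigger actor that completes a quest when the player character reaches it.
; On box overlap, it scans the character's active quests for any whose actor reference is this actor and calls QuestComplete on the character.
; It then searches all BP_Xipsy actors and fires EventQuestComplete on those whose quest name matches the completed quest.
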(event OnComponentBeginOverlap(Box)
  (params (OverlappedComponent :type Primitive%20Component%20Object%20Reference) (OtherActor :type Actor%20Object%20Reference) (OtherComp :type Primitive%20Component%20Object%20Reference) (OtherBodyIndex :type Integer) (bFromSweep :type Boolean) (SweepResult :type Hit%20Result%20Structure%20%28by%20ref%29))
  (bind _asbp_third_person_character (Utilities|Casting|CastToBP_ThirdPersonCharacter OtherActor))
  (for _array_element (Variables|/Game/ThirdPerson/Blueprints/BP_ThirdPersonCharacter.BP_ThirdPersonCharacter_C|GetActiveQuests _asbp_third_person_character)
    (if (== self (.actorreference (Variables|/Game/Nathan/Dialogue_Quests/BP_Quest.BP_Quest_C|GetQuestInfo _array_element)))
      (Default|QuestComplete _asbp_third_person_character _array_element)
      (bind _outactors (Actor|GetAllActorsOfClass "/Game/Nathan/Dialogue_Quests/BP_Xipsy.BP_Xipsy_C"))
      (for _array_element_2 _outactors
        (if (Utilities|Enum|Equal(Enum) (.questname (Variables|/Game/Nathan/Dialogue_Quests/BP_Quest.BP_Quest_C|GetQuestInfo _array_element)) (.questname (Variables|/Game/Nathan/Dialogue_Quests/BP_Xipsy.BP_Xipsy_C|GetQuestRef _array_element_2)))
          (Default|EventQuestComplete _array_element_2))))))

(fn ConstructionScript)