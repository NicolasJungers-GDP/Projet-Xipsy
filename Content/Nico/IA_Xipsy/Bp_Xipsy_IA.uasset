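; Xipsy AI companion Blueprint that follows the player character.
; BeginPlay caches the player as BP_ThirdPersonCharacter and starts FollowPlayer, which re-runs itself after a short delay following each move request.
; While the follow flag is set, it uses AIMoveTo toward the player when far enough away, otherwise targets itself to halt.
; StopMouvement jumps into that same halt branch, which also re-enters the loop.
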(event Custom|Follow%20Player
  (if (Variables|Default|GetFollowPlayer?)
    (if (>= (Transformation|GetDistanceTo (Variables|Default|GetCharacter%20Ref)) 4e+02)
      (AI|AIMoveTo self "0, 0, 0" (Variables|Default|GetCharacter%20Ref) 5.0 false
        (:then
          _))
      (else
        (AI|AIMoveTo self "0, 0, 0" self 5.0 false
          (:then
            _))))
    (Utilities|FlowControl|Delay 0.2)
    (CallFunction|FollowPlayer)))

(event Custom|Stop%20Mouvement
  (AI|AIMoveTo self "0, 0, 0" self 5.0 false
    (:then
      (Utilities|FlowControl|Delay 0.2)
      (CallFunction|FollowPlayer))))

(event EventBeginPlay
  (bind _asbp_third_person_character (Utilities|Casting|CastToBP_ThirdPersonCharacter (Game|GetPlayerCharacter 0)))
  (Variables|Default|SetCharacter%20Ref _asbp_third_person_character)
  (CallFunction|FollowPlayer))

(fn ConstructionScript)